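; Third-person shooter character Blueprint that creates the player's HUD and keeps its health display current.
; BeginPlay creates the HUD widget and adds it to the viewport, and Tick copies TPSHealth's health into it every frame rather than on damage events.
; Unconnected nodes hold weapon spawning with attachment to the mesh's WeaponSocket, plus placeholder setters for clip and total ammo on the HUD, so none of these run.
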(event `self.ReceiveTick`
  (params (DeltaSeconds :type "Float (single-precision)"))
  ;[0.5836 1 0.4491] this is just passing over the health each frame, if I had an event for taking damage, that could be done there aswell <3
  (set `/Game/UI/HUD.PlayerHealth` (`TPSHealthComponent.health` (`self.TPSHealth`)) (`self.HUD`)))

(event `self.ReceiveBeginPlay`
  (bind _returnvalue (`|CreateWidget` "/Game/UI/HUD.HUD_C"))
  (bind _output_get (set `self.HUD` _returnvalue))
  (`UserWidget.AddToViewport` _returnvalue 0)
  (`UserWidget.AddToViewport` _output_get 0))

(fn `UserConstructionScript`)